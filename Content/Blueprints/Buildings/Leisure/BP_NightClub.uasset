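; BP_NightClub is a leisure building that serves as a nightclub with a capped number of visitors.
; BeginPlay sets the visitor limit, and every Tick polls IsOpen and copies the result to the Enabled flag of four BP_DiscoLight child actors.
; The EnableRoof event shows or hides the roof mesh and its child components.
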(event EventBeginPlay
  (Class|BuildingBase|SetMaxVisitors 8))

(event Collision|EventActorBeginOverlap
  (params (OtherActor :type Actor%20Object%20Reference)))

(event EventTick
  (params (DeltaSeconds :type Float%20%28single-precision%29))
  (bind _returnvalue (Class|BuildingBase|IsOpen))
  (bind _asbp_disco_light (Utilities|Casting|CastToBP_DiscoLight (Variables|/Script/Engine.ChildActorComponent|GetChildActor (Variables|Default|GetChildActor10))))
  (Variables|/Game/Blueprints/model/BP_DiscoLight.BP_DiscoLight_C|Setenabled _asbp_disco_light _returnvalue)
  (bind _asbp_disco_light_2 (Utilities|Casting|CastToBP_DiscoLight (Variables|/Script/Engine.ChildActorComponent|GetChildActor (Variables|Default|GetChildActor11))))
  (Variables|/Game/Blueprints/model/BP_DiscoLight.BP_DiscoLight_C|Setenabled _asbp_disco_light_2 _returnvalue)
  (bind _asbp_disco_light_3 (Utilities|Casting|CastToBP_DiscoLight (Variables|/Script/Engine.ChildActorComponent|GetChildActor (Variables|Default|GetChildActor12))))
  (Variables|/Game/Blueprints/model/BP_DiscoLight.BP_DiscoLight_C|Setenabled _asbp_disco_light_3 _returnvalue)
  (bind _asbp_disco_light_4 (Utilities|Casting|CastToBP_DiscoLight (Variables|/Script/Engine.ChildActorComponent|GetChildActor (Variables|Default|GetChildActor9))))
  (Variables|/Game/Blueprints/model/BP_DiscoLight.BP_DiscoLight_C|Setenabled _asbp_disco_light_4 _returnvalue))

(event EventEnableRoof
  (params (enable :type Boolean))
  (Rendering|SetVisibility (Variables|Default|GetStaticMesh10) enable true))

(fn ConstructionScript)