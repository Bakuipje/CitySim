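; Railroad building actor that lays track along a Spline as a chain of spline mesh components, one per pair of neighboring points.
; The construction script creates and attaches each segment using local point positions and tangents, so the track follows the curve.
; BeginPlay repeats the loop to add another set of segments, but passes only start and end positions, leaving tangents unset.
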(event EventBeginPlay
  (for _index (range 0 (- (Spline|GetNumberOfSplinePoints (Variables|Default|GetSpline)) 2))
    (bind _returnvalue (AddComponent|AddSplineMeshComponent false))
    (Variables|Default|SetNewVar_0 _returnvalue)
    (SplineMesh|SetForwardAxis (Variables|Default|GetNewVar_0) (Variables|Default|Getforward%20axis) true)
    (Transformation|AttachComponentToComponent (Variables|Default|GetNewVar_0) (Variables|Default|GetSpline) "None" "KeepRelative" "KeepRelative" "KeepRelative" true)
    (SplineMesh|SetStartandEnd (Variables|Default|GetNewVar_0) (Spline|GetLocationatSplinePoint (Variables|Default|GetSpline) _index "Local") "0, 0, 0" (Spline|GetLocationatSplinePoint (Variables|Default|GetSpline) (+ _index 1) "Local") "0, 0, 0" true :!class /Script/Engine.SplineMeshComponent)))

(event Collision|EventActorBeginOverlap
  (params (OtherActor :type Actor%20Object%20Reference)))

(event EventTick
  (params (DeltaSeconds :type Float%20%28single-precision%29)))

(fn ConstructionScript
  (bind _spline (Variables|Default|GetSpline))
  (bind _spline_2 (Variables|Default|GetSpline))
  (for _index (range 0 (- (Spline|GetNumberOfSplinePoints (Variables|Default|GetSpline)) 2))
    (bind _returnvalue (AddComponent|AddSplineMeshComponent true))
    (Variables|Default|SetNewVar_0 _returnvalue)
    (SplineMesh|SetForwardAxis (Variables|Default|GetNewVar_0) (Variables|Default|Getforward%20axis) true)
    (Transformation|AttachComponentToComponent (Variables|Default|GetNewVar_0) (Variables|Default|GetSpline) "None" "KeepRelative" "KeepRelative" "KeepRelative" true)
    (SplineMesh|SetStartandEnd (Variables|Default|GetNewVar_0) (Spline|GetLocationatSplinePoint _spline_2 _index "Local") (Spline|GetTangentatSplinePoint _spline_2 _index "Local") (Spline|GetLocationatSplinePoint _spline (+ _index 1) "Local") (Spline|GetTangentatSplinePoint _spline (+ _index 1) "Local") true :!class /Script/Engine.SplineMeshComponent)))