(event OnComponentBeginOverlap(CapsuleComponent)
  (params (OverlappedComponent :type Primitive%20Component%20Object%20Reference) (OtherActor :type Actor%20Object%20Reference) (OtherComp :type Primitive%20Component%20Object%20Reference) (OtherBodyIndex :type Integer) (bFromSweep :type Boolean) (SweepResult :type Hit%20Result%20Structure%20%28by%20ref%29))
  (bind _asbp_agent (Utilities|Casting|CastToBP_agent OtherActor))
  (Class|Agent|AttackAgent _asbp_agent))

(event EventBeginPlay
  (bind _goap (Variables|Default|GetGoap))
  (bind _goapactions (Variables|/Script/Simulation.GoapComponent|GetgoapActions _goap))
  (CallFunction|FindMoodUI)
  (Class|Agent|EnableArrowVisual false)
  (bind _returnvalue (Game|ConstructObjectfromClass "/Game/Blueprints/Moods/BP_Work.BP_Work_C" self))
  (CallFunction|FindMoodUI)
  (bind _returnvalue_2 (Game|ConstructObjectfromClass "/Game/Blueprints/Moods/BP_homemood.BP_homemood_C" self))
  (Utilities|Array|Add (Variables|/Script/Simulation.MoodComponent|Getm_moods (Variables|Default|GetMood)) _returnvalue_2)
  (Variables|Default|Setworkmood _returnvalue)
  (bind _returnvalue_3 (Game|ConstructObjectfromClass "/Game/Blueprints/Moods/BP_Liesure.BP_Liesure_C" self))
  (Variables|Default|SetstressMood _returnvalue_3)
  (bind _returnvalue_4 (Game|ConstructObjectfromClass "/Game/Blueprints/Moods/BP_FoodMood.BP_FoodMood_C" self))
  (Variables|Default|SetfoodMood _returnvalue_4)
  (bind _returnvalue_5 (Game|ConstructObjectfromClass "/Script/Simulation.GymMood" self))
  (Variables|Default|SetgymMood _returnvalue_5)
  (bind _returnvalue_6 (Game|ConstructObjectfromClass "/Script/Simulation.FindWater" self))
  (Utilities|Array|Add _goapactions _returnvalue_6)
  (bind _returnvalue_7 (Game|ConstructObjectfromClass "/Script/Simulation.WaterPlant" self))
  (Utilities|Array|Add _goapactions _returnvalue_7))

(event Collision|EventActorBeginOverlap
  (params (OtherActor :type Actor%20Object%20Reference)))

(event EventTick
  (params (DeltaSeconds :type Float%20%28single-precision%29))
  (if (Utilities|IsValid (Variables|Default|GetuiMood))
    _
    (else
      (CallFunction|FindMoodUI)))
  (if (Variables|Default|Getclicked)
    (Class|Agent|EnableArrowVisual true)
    (CallFunction|AddListItems)))

(event MouseInput|EventActorOnClicked
  (params (ButtonPressed :type Key%20Structure))
  (if (== ButtonPressed "RightMouseButton")
    (Variables|Default|SetRightClick true)
    (else
      (Variables|Default|SetRightClick false)))
  (CallFunction|ResetClicable)
  (bind _asdata_visualizer (Utilities|Casting|CastTodataVisualizer (Variables|Default|GetuiMood))
    (:then
      (Default|ClearVisibility _asdata_visualizer))
    (:CastFailed
      _))
  (Variables|Default|Setclicked true)
  (bind _output_get (Variables|Default|Setbody%20col "(R=0.098297,G=0.000000,B=1.000000,A=1.000000)"))
  (Rendering|Material|SetVectorParameterValue (Variables|Default|GetmaterialInstance) "BodyColor" _output_get :!class /Script/Engine.MaterialInstanceDynamic))

(event EventEnableArrowVisual
  (params (enable :type Boolean))
  (Rendering|SetVisibility (Variables|Default|GetStaticMesh) enable true))

(fn ConstructionScript
  (bind _returnvalue (Rendering|Material|CreateDynamicMaterialInstance (Variables|Character|GetMesh) 0 "/Game/Mannequin/Character/Materials/M_UE4Man_Body.M_UE4Man_Body" :!class /Script/Engine.PrimitiveComponent))
  (Variables|Default|SetmaterialInstance _returnvalue)
  (Rendering|Material|SetVectorParameterValue _returnvalue "BodyColor" (Variables|Default|Getbody%20col) :!class /Script/Engine.MaterialInstanceDynamic))

(fn FindMoodUI
  (bind _outactors (Actor|GetAllActorsOfClass "/Game/Blueprints/World/BP_WorldRules.BP_WorldRules_C"))
  (for _array_element _outactors
    (bind _asdata_visualizer (Utilities|Casting|CastTodataVisualizer (Variables|/Script/Simulation.WorldRules|GetdataVisualizerWidget _array_element)))
    (Variables|Default|SetuiMood _asdata_visualizer)
    (return)))

(fn AddListItems
  (bind _returnvalue (Class|Agent|GetActorStringStats))
  (bind _asdata_visualizer (Utilities|Casting|CastTodataVisualizer (Variables|Default|GetuiMood)))
  (Rendering|Components|TextRender|SetText (Variables|/Game/Widgets/dataVisualizer.dataVisualizer_C|GetTextBlock_2 _asdata_visualizer) (Utilities|Text|ToText(String) _returnvalue))
  (Widget|Panel|ClearChildren (Variables|/Game/Widgets/dataVisualizer.dataVisualizer_C|GetMoodList _asdata_visualizer))
  (if (Variables|Default|GetRightClick)
    (bind _asdata_visualizer_2 (Utilities|Casting|CastTodataVisualizer (Variables|Default|GetuiMood)))
    (bind _returnvalue_2 (Class|Agent|GetActorRelationStringStats (Variables|/Game/Widgets/dataVisualizer.dataVisualizer_C|GetShowStrings _asdata_visualizer_2)))
    (bind _asdata_visualizer_3 (Utilities|Casting|CastTodataVisualizer (Variables|Default|GetuiMood)))
    (Default|CreateandAddChild _asdata_visualizer_3 _returnvalue_2)
    (else
      (bind _returnvalue_3 (Class|MoodComponent|GetThinkingString (Variables|Default|GetMood)))
      (bind _asdata_visualizer_4 (Utilities|Casting|CastTodataVisualizer (Variables|Default|GetuiMood)))
      (Default|CreateandAddChild _asdata_visualizer_4 _returnvalue_3)))
  (return))

(fn CreateandSetText
  (params (NewParam :type String))
  (bind _returnvalue (UserInterface|CreateWidget "/Game/Widgets/ListButton.ListButton_C" (Game|GetPlayerController 0)))
  (Variables|/Game/Widgets/ListButton.ListButton_C|SetText%20To%20Display _returnvalue NewParam)
  (Rendering|Components|TextRender|SetText (Variables|/Game/Widgets/ListButton.ListButton_C|GetMoodText _returnvalue) (Utilities|Text|ToText(String) NewParam))
  (return _returnvalue))

(fn ResetClicable
  (Class|DataVisualizerWidget|ClearMoodList (Variables|Default|GetuiMood))
  (bind _outactors (Actor|GetAllActorsOfClass "BP_agent_C"))
  (for _array_element _outactors
    (bind _asbp_agent (Utilities|Casting|CastToBP_agent _array_element))
    (Class|Agent|EnableArrowVisual _asbp_agent false)
    (Variables|/Script/Simulation.Agent|Setclicked _asbp_agent false)
    (bind _returnvalue (Class|RelationComponent|GetFriendlyValue (Variables|Default|GetRelation) _asbp_agent))
    (bind _newparam (CallFunction|GetEmotionColor _returnvalue))
    (Rendering|Material|SetVectorParameterValue (Variables|BP_agent_C|GetmaterialInstance _asbp_agent) "BodyColor" _newparam :!class /Script/Engine.MaterialInstanceDynamic)))

(fn GetEmotionColor
  (params (NewParam1 :type Float%20%28single-precision%29))
  (bind _returnvalue (- 1.0 NewParam1))
  (bind _returnvalue_2 (+ NewParam1 1.0))
  (if (>= NewParam1 0.0)
    (LocalVariables|SetNewLocalVar_0 (Utilities|Struct|MakeLinearColor _returnvalue 1.0 _returnvalue 1.0))
    (else
      (LocalVariables|SetNewLocalVar_0 (Utilities|Struct|MakeLinearColor 1.0 _returnvalue_2 _returnvalue_2 1.0))))
  (return (LocalVariables|GetNewLocalVar_0)))

(fn DrawLine
  (params (NewParam :type Agent%20Object%20Reference))
  (Rendering|Debug|DrawDebugLine (Transformation|GetActorLocation) (Transformation|GetActorLocation NewParam) "(R=1.000000,G=0.000000,B=0.933392,A=1.000000)" 0.0 1e+01))