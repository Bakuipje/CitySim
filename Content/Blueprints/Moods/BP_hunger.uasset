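; Hunger mood Blueprint that builds and starts the behavior tree for finding and eating food.
; GetBehaviorTree constructs the tree at runtime from behavior objects, under a costed RGQueue root bound to the passed component.
; The queue holds an eat behavior, then a sequence that finds FoodBase consumables in range, moves to one, picks it up, eats and runs a timer.
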(fn GetBehaviorTree
  (params (behviorTreeComponent :type RG%20Behavior%20Tree%20Component%20Object%20Reference))
  (bind _returnvalue (Game|ConstructObjectfromClass "/Script/Simulation.RGQueue" self))
  (Variables|/Script/Simulation.RGBehaviorTreeBase|Setm_cost _returnvalue 2)
  (bind _output_get (Variables|Default|SetbehaviorTree _returnvalue))
  (bind _returnvalue_2 (Game|ConstructObjectfromClass "/Script/Simulation.EatBehavior" self))
  (Variables|/Script/Simulation.EatBehavior|Setm_moodType _returnvalue_2 "BP_hunger_C")
  (bind _returnvalue_3 (Game|ConstructObjectfromClass "/Script/Simulation.RGSequence" self))
  (bind _returnvalue_4 (Game|ConstructObjectfromClass "/Script/Simulation.FindConsumable" self))
  (Variables|/Script/Simulation.FindConsumable|Setm_invertoryType _returnvalue_4 "/Script/Simulation.FoodBase")
  (Variables|/Script/Simulation.FindConsumable|Setm_range _returnvalue_4 2e+02)
  (bind _returnvalue_5 (Game|ConstructObjectfromClass "/Game/Blueprints/BP_MoveToInteractable.BP_MoveToInteractable_C" self))
  (Variables|/Game/Blueprints/BP_MoveToInteractable.BP_MoveToInteractable_C|Setrange _returnvalue_5 2e+02)
  (bind _returnvalue_6 (Game|ConstructObjectfromClass "/Script/Simulation.PickConsumable" self))
  (Variables|/Script/Simulation.PickConsumable|Setm_invertoryType _returnvalue_6 "/Script/Simulation.FoodBase")
  (bind _returnvalue_7 (Game|ConstructObjectfromClass "/Script/Simulation.EatBehavior" self))
  (Variables|/Script/Simulation.EatBehavior|Setm_moodType _returnvalue_7 "BP_hunger_C")
  (bind _returnvalue_8 (Game|ConstructObjectfromClass "/Script/Simulation.RGTimer" self))
  (Variables|/Script/Simulation.RGTimer|Setm_time _returnvalue_8 4.0)
  (Utilities|Array|Add (Variables|/Script/Simulation.RGBehaviorTreeBase|Getm_behaviorList _output_get) _returnvalue_2)
  (Utilities|Array|Add (Variables|/Script/Simulation.RGBehaviorTreeBase|Getm_behaviorList _output_get) _returnvalue_3)
  (Utilities|Array|Add (Variables|/Script/Simulation.RGBehaviorTreeBase|Getm_behaviorList _returnvalue_3) _returnvalue_4)
  (Utilities|Array|Add (Variables|/Script/Simulation.RGBehaviorTreeBase|Getm_behaviorList _returnvalue_3) _returnvalue_5)
  (Utilities|Array|Add (Variables|/Script/Simulation.RGBehaviorTreeBase|Getm_behaviorList _returnvalue_3) _returnvalue_6)
  (Utilities|Array|Add (Variables|/Script/Simulation.RGBehaviorTreeBase|Getm_behaviorList _returnvalue_3) _returnvalue_7)
  (Utilities|Array|Add (Variables|/Script/Simulation.RGBehaviorTreeBase|Getm_behaviorList _returnvalue_3) _returnvalue_8)
  (Variables|/Script/Simulation.RGBehaviorTreeBase|Setm_ownerComp (Variables|Default|GetbehaviorTree) behviorTreeComponent)
  (Class|RGBehaviorTreeBase|BeginPlay (Variables|Default|GetbehaviorTree))
  (return _output_get))