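; BP_openDoor is a mood that builds an AI behavior tree for opening a door, fetching a key first if needed.
; GetBehaviorTree constructs the RG nodes at runtime under a root selector, starts it with BeginPlay and returns it.
; A domain conditioned on holding BP_key runs a find, move and open-door sequence.
; The fallback sequence finds and picks up a key, then nests the same door sequence.
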(fn GetBehaviorTree
  (params (behviorTreeComponent :type RG%20Behavior%20Tree%20Component%20Object%20Reference))
  (bind _returnvalue (Game|ConstructObjectfromClass "/Script/Simulation.RGSelector" behviorTreeComponent))
  (Variables|/Script/Simulation.RGBehaviorTreeBase|Setm_ownerComp _returnvalue behviorTreeComponent)
  (bind _behaviortree (CallFunction|HasType behviorTreeComponent _returnvalue))
  (CallFunction|MovetoObstacle behviorTreeComponent _behaviortree)
  (bind _output_node (CallFunction|FindKey behviorTreeComponent _returnvalue))
  (CallFunction|MovetoObstacle behviorTreeComponent _output_node)
  (Class|RGBehaviorTreeBase|BeginPlay _returnvalue)
  (return _returnvalue))

(fn HasType
  (params (NewParam :type RG%20Behavior%20Tree%20Component%20Object%20Reference) (parentNode :type RG%20Behavior%20Tree%20Base%20Object%20Reference))
  (bind _returnvalue (Game|ConstructObjectfromClass "/Script/Simulation.RGDomain" NewParam))
  (Utilities|Array|Add (Variables|/Script/Simulation.RGBehaviorTreeBase|Getm_behaviorList parentNode) _returnvalue)
  (bind _returnvalue_2 (Game|ConstructObjectfromClass "/Script/Simulation.HasConsumable" NewParam))
  (Variables|/Script/Simulation.HasConsumable|Setm_inventoryType _returnvalue_2 "/Game/Blueprints/interactables/Consumables/BP_key.BP_key_C")
  (Utilities|Array|Add (Variables|/Script/Simulation.RGDomain|Getm_conditions _returnvalue) _returnvalue_2)
  (return _returnvalue))

(fn MovetoObstacle
  (params (behaviortreeCOmp :type RG%20Behavior%20Tree%20Component%20Object%20Reference) (ParentNode :type RG%20Behavior%20Tree%20Base%20Object%20Reference))
  (bind _returnvalue (Game|ConstructObjectfromClass "/Script/Simulation.RGSequence" behaviortreeCOmp))
  (Utilities|Array|Add (Variables|/Script/Simulation.RGBehaviorTreeBase|Getm_behaviorList ParentNode) _returnvalue)
  (bind _returnvalue_2 (Game|ConstructObjectfromClass "/Script/Simulation.FindStorage" behaviortreeCOmp))
  (Variables|/Script/Simulation.FindStorage|Setm_storageType _returnvalue_2 "/Game/Blueprints/interactables/Storage/BP_Door.BP_Door_C")
  (Variables|/Script/Simulation.FindStorage|Setm_range _returnvalue_2 1e+05)
  (Utilities|Array|Add (Variables|/Script/Simulation.RGBehaviorTreeBase|Getm_behaviorList _returnvalue) _returnvalue_2)
  (bind _returnvalue_3 (Game|ConstructObjectfromClass "/Script/Simulation.MoveToInteractable" behaviortreeCOmp))
  (Variables|/Script/Simulation.MoveToInteractable|Setm_range _returnvalue_3 1e+02)
  (Utilities|Array|Add (Variables|/Script/Simulation.RGBehaviorTreeBase|Getm_behaviorList _returnvalue) _returnvalue_3)
  (bind _returnvalue_4 (Game|ConstructObjectfromClass "/Game/Blueprints/Behaviors/BP_openDoorBehavior.BP_openDoorBehavior_C" behaviortreeCOmp))
  (Utilities|Array|Add (Variables|/Script/Simulation.RGBehaviorTreeBase|Getm_behaviorList _returnvalue) _returnvalue_4)
  (return _returnvalue))

(fn FindKey
  (params (behavior%20tree%20component :type RG%20Behavior%20Tree%20Component%20Object%20Reference) (parent%20Node :type RG%20Behavior%20Tree%20Base%20Object%20Reference))
  (bind _returnvalue (Game|ConstructObjectfromClass "/Script/Simulation.RGSequence" behavior%20tree%20component))
  (Utilities|Array|Add (Variables|/Script/Simulation.RGBehaviorTreeBase|Getm_behaviorList parent%20Node) _returnvalue)
  (bind _returnvalue_2 (Game|ConstructObjectfromClass "/Script/Simulation.FindConsumable" behavior%20tree%20component))
  (Variables|/Script/Simulation.FindConsumable|Setm_invertoryType _returnvalue_2 "/Game/Blueprints/interactables/Consumables/BP_key.BP_key_C")
  (Variables|/Script/Simulation.FindConsumable|Setm_range _returnvalue_2 1e+04)
  (Utilities|Array|Add (Variables|/Script/Simulation.RGBehaviorTreeBase|Getm_behaviorList _returnvalue) _returnvalue_2)
  (bind _returnvalue_3 (Game|ConstructObjectfromClass "/Script/Simulation.MoveToInteractable" behavior%20tree%20component))
  (Variables|/Script/Simulation.MoveToInteractable|Setm_range _returnvalue_3 1e+02)
  (Utilities|Array|Add (Variables|/Script/Simulation.RGBehaviorTreeBase|Getm_behaviorList _returnvalue) _returnvalue_3)
  (bind _returnvalue_4 (Game|ConstructObjectfromClass "/Script/Simulation.PickConsumable" behavior%20tree%20component))
  (Variables|/Script/Simulation.PickConsumable|Setm_invertoryType _returnvalue_4 "/Game/Blueprints/interactables/Consumables/BP_key.BP_key_C")
  (Utilities|Array|Add (Variables|/Script/Simulation.RGBehaviorTreeBase|Getm_behaviorList _returnvalue) _returnvalue_4)
  (return _returnvalue))