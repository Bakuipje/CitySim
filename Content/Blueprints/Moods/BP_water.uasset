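; Water mood that builds a behavior tree in Blueprint for an agent to fetch water and water flowers.
; A root selector tries delivery first, gated on carried water and a path to current storage, then falls back to a find-and-pick-up sequence.
; That fallback includes a path check carrying an open-door mood and ends with a second copy of the delivery branch.
; AddFindKey is defined but not called here.
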(fn GetBehaviorTree
  (params (behviorTreeComponent :type RG%20Behavior%20Tree%20Component%20Object%20Reference))
  (bind _returnvalue (Game|ConstructObjectfromClass "/Script/Simulation.RGSelector" behviorTreeComponent))
  (Variables|/Script/Simulation.RGBehaviorTreeBase|Setm_ownerComp _returnvalue behviorTreeComponent)
  (CallFunction|MovetoWaterDestination behviorTreeComponent _returnvalue)
  (bind _behaviortreenode (CallFunction|MovetoWaterSource behviorTreeComponent _returnvalue))
  (bind _newparam1 (CallFunction|MovetoWaterDestination behviorTreeComponent _behaviortreenode))
  (Class|RGBehaviorTreeBase|BeginPlay _behaviortreenode)
  (return _returnvalue))

(fn MovetoWaterSource
  (params (behaviortreecomp :type RG%20Behavior%20Tree%20Component%20Object%20Reference) (parentNode :type RG%20Behavior%20Tree%20Base%20Object%20Reference))
  (bind _returnvalue (Game|ConstructObjectfromClass "/Script/Simulation.RGSequence" behaviortreecomp))
  (bind _returnvalue_2 (Game|ConstructObjectfromClass "/Script/Simulation.FindConsumable" behaviortreecomp))
  (Variables|/Script/Simulation.FindConsumable|Setm_invertoryType _returnvalue_2 "/Game/Blueprints/interactables/Consumables/BP_waterConsumable.BP_waterConsumable_C")
  (Variables|/Script/Simulation.FindConsumable|Setm_range _returnvalue_2 1e+03)
  (bind _newparam1 (CallFunction|HasPath behaviortreecomp))
  (bind _returnvalue_3 (Game|ConstructObjectfromClass "/Script/Simulation.MoveToInteractable" behaviortreecomp))
  (Variables|/Script/Simulation.MoveToInteractable|Setm_range _returnvalue_3 3e+02)
  (bind _returnvalue_4 (Game|ConstructObjectfromClass "/Script/Simulation.PickConsumable" behaviortreecomp))
  (Variables|/Script/Simulation.PickConsumable|Setm_invertoryType _returnvalue_4 "/Game/Blueprints/interactables/Consumables/BP_waterConsumable.BP_waterConsumable_C")
  (Utilities|Array|Add (Variables|/Script/Simulation.RGBehaviorTreeBase|Getm_behaviorList _returnvalue) _returnvalue_2)
  (Utilities|Array|Add (Variables|/Script/Simulation.RGBehaviorTreeBase|Getm_behaviorList _returnvalue) _newparam1)
  (Utilities|Array|Add (Variables|/Script/Simulation.RGBehaviorTreeBase|Getm_behaviorList _returnvalue) _returnvalue_3)
  (Utilities|Array|Add (Variables|/Script/Simulation.RGBehaviorTreeBase|Getm_behaviorList _returnvalue) _returnvalue_4)
  (Utilities|Array|Add (Variables|/Script/Simulation.RGBehaviorTreeBase|Getm_behaviorList parentNode) _returnvalue)
  (return _returnvalue))

(fn MovetoWaterDestination
  (params (NewParam :type RG%20Behavior%20Tree%20Component%20Object%20Reference) (parent :type RG%20Behavior%20Tree%20Base%20Object%20Reference))
  (bind _conditions (CallFunction|HasInventory NewParam))
  (bind _returnvalue (Game|ConstructObjectfromClass "/Script/Simulation.RGSequence" NewParam))
  (Utilities|Array|Add (Variables|/Script/Simulation.RGBehaviorTreeBase|Getm_behaviorList _conditions) _returnvalue)
  (bind _returnvalue_2 (Game|ConstructObjectfromClass "/Script/Simulation.FindStorage" NewParam))
  (Variables|/Script/Simulation.FindStorage|Setm_storageType _returnvalue_2 "/Game/Blueprints/interactables/Storage/BP_Flower.BP_Flower_C")
  (bind _returnvalue_3 (Game|ConstructObjectfromClass "/Script/Simulation.MoveToInteractable" NewParam))
  (Variables|/Script/Simulation.MoveToInteractable|Setm_range _returnvalue_3 3e+02)
  (bind _returnvalue_4 (Game|ConstructObjectfromClass "/Game/Blueprints/Behaviors/BP_WaterPlant.BP_WaterPlant_C" NewParam))
  (Utilities|Array|Add (Variables|/Script/Simulation.RGBehaviorTreeBase|Getm_behaviorList _returnvalue) _returnvalue_2)
  (Utilities|Array|Add (Variables|/Script/Simulation.RGBehaviorTreeBase|Getm_behaviorList _returnvalue) _returnvalue_3)
  (Utilities|Array|Add (Variables|/Script/Simulation.RGBehaviorTreeBase|Getm_behaviorList _returnvalue) _returnvalue_4)
  (Utilities|Array|Add (Variables|/Script/Simulation.RGBehaviorTreeBase|Getm_behaviorList parent) _conditions)
  (return parent))

(fn HasInventory
  (params (NewParam :type RG%20Behavior%20Tree%20Component%20Object%20Reference))
  (bind _returnvalue (Components|GetOwner NewParam))
  (bind _returnvalue_2 (Game|ConstructObjectfromClass "/Script/Simulation.RGDomain" NewParam))
  (bind _returnvalue_3 (Game|ConstructObjectfromClass "/Script/Simulation.HasConsumable" NewParam))
  (Variables|/Script/Simulation.HasConsumable|Setm_inventoryType _returnvalue_3 "/Game/Blueprints/interactables/Consumables/BP_waterConsumable.BP_waterConsumable_C")
  (Utilities|Array|Add (Variables|/Script/Simulation.RGDomain|Getm_conditions _returnvalue_2) _returnvalue_3)
  (bind _returnvalue_4 (Game|ConstructObjectfromClass "/Script/Simulation.RGHasPath" NewParam))
  (bind _asagent (Utilities|Casting|CastToAgent _returnvalue))
  (Variables|/Script/Simulation.RGHasPath|Setagent _returnvalue_4 _asagent)
  (Variables|/Script/Simulation.RGHasPath|SetstartLocation _returnvalue_4 (Transformation|GetActorLocation _returnvalue))
  (Variables|/Script/Simulation.RGHasPath|SetendLocation _returnvalue_4 (Transformation|GetActorLocation (Variables|/Script/Simulation.Agent|GetcurrentStorage _asagent)))
  (Utilities|Array|Add (Variables|/Script/Simulation.RGDomain|Getm_conditions _returnvalue_2) _returnvalue_4)
  (return _returnvalue_2))

(fn HasPath
  (params (NewParam :type RG%20Behavior%20Tree%20Component%20Object%20Reference))
  (bind _returnvalue (Components|GetOwner NewParam))
  (bind _returnvalue_2 (Game|ConstructObjectfromClass "/Script/Simulation.RGDomain" NewParam))
  (bind _returnvalue_3 (Game|ConstructObjectfromClass "/Script/Simulation.RGHasPath" NewParam))
  (bind _returnvalue_4 (Game|ConstructObjectfromClass "/Game/Blueprints/Moods/BP_openDoor.BP_openDoor_C" NewParam))
  (Variables|/Script/Simulation.RGHasPath|Setmood _returnvalue_3 _returnvalue_4)
  (bind _asbp_agent (Utilities|Casting|CastToBP_agent _returnvalue)
    (:then
      (Variables|/Script/Simulation.RGHasPath|Setagent _returnvalue_3 _asbp_agent)
      (Utilities|IsValid (Variables|/Script/Simulation.Agent|GetcurrentStorage _asbp_agent)
        (:Is%20Valid
          (Variables|/Script/Simulation.RGHasPath|SetstartLocation _returnvalue_3 (Transformation|GetActorLocation _returnvalue))
          (Variables|/Script/Simulation.RGHasPath|SetendLocation _returnvalue_3 (Transformation|GetActorLocation (Variables|/Script/Simulation.Agent|GetcurrentStorage _asbp_agent))))
        (:Is%20Not%20Valid
          _)))
    (:CastFailed
      _))
  (Utilities|Array|Add (Variables|/Script/Simulation.RGDomain|Getm_conditions _returnvalue_2) _returnvalue_3)
  (return _returnvalue_2))

(fn AddFindKey
  (params (NewParam :type RG%20Behavior%20Tree%20Component%20Object%20Reference) (parentNode :type RG%20Behavior%20Tree%20Base%20Object%20Reference))
  (bind _returnvalue (Game|ConstructObjectfromClass "/Game/Blueprints/Behaviors/BP_addopenDoor.BP_addopenDoor_C" NewParam))
  (Utilities|Array|Add (Variables|/Script/Simulation.RGBehaviorTreeBase|Getm_behaviorList parentNode) _returnvalue)
  (return _returnvalue))