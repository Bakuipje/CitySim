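; BP_MoveToInteractable is a behavior node that walks an Agent to its current storage actor.
; Each Tick compares squared distance to the storage against squared Range, issuing MoveTo and returning Progress while at or beyond it, and Succeed once inside.
; It returns Failed when the owner is not an Agent or has no valid CurrentStorage.
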(fn Tick
  (params (deltaTime :type Float%20%28single-precision%29))
  (bind _range (Variables|Default|Getrange))
  (bind _m_ownercomp (Variables|Default|Getm_ownerComp))
  (bind _returnvalue (Components|GetOwner _m_ownercomp))
  (bind _asagent (Utilities|Casting|CastToAgent _returnvalue)
    (:then
      (if (Utilities|IsValid (Variables|/Script/Simulation.Agent|GetcurrentStorage _asagent))
        (if (>= (Math|Vector|VectorLengthSquared (- (Transformation|GetActorLocation (Variables|/Script/Simulation.Agent|GetcurrentStorage _asagent)) (Transformation|GetActorLocation _returnvalue))) (* _range _range))
          (Class|Agent|Moveto _asagent (Transformation|GetActorLocation (Variables|/Script/Simulation.Agent|GetcurrentStorage _asagent)))
          (bind _output_get (Variables|Default|SetbehaviorState "EB_Progress"))
          (return _output_get)
          (else
            (bind _output_get_2 (Variables|Default|SetbehaviorState "EB_Succeed"))
            (return _output_get_2)))
        (else
          _)))
    (:CastFailed
      _))
  (bind _output_get_3 (Variables|Default|SetbehaviorState "EB_Failed"))
  (return _output_get_3))