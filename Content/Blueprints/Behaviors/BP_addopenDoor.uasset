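; BP_addopenDoor is a behavior that adds a BP_openDoor mood to the owning actor's MoodComponent.
; Tick scans MMoods and, at the first entry of another class, constructs a BP_openDoor, appends it and returns Succeed.
; The check is per entry, so it can add duplicates, and an empty list gains nothing but still succeeds.
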(fn Tick
  (params (deltaTime :type Float%20%28single-precision%29))
  (bind _m_ownercomp (Variables|Default|Getm_ownerComp))
  (bind _returnvalue (Components|GetOwner _m_ownercomp))
  (bind _returnvalue_2 (Actor|GetComponentbyClass _returnvalue "/Script/Simulation.MoodComponent"))
  (bind _m_moods (Variables|/Script/Simulation.MoodComponent|Getm_moods _returnvalue_2))
  (for _array_element _m_moods
    (if (not (== (Utilities|GetClass _array_element) "/Game/Blueprints/Moods/BP_openDoor.BP_openDoor_C"))
      (bind _returnvalue_3 (Game|ConstructObjectfromClass "/Game/Blueprints/Moods/BP_openDoor.BP_openDoor_C" _m_ownercomp))
      (Utilities|Array|Add _m_moods _returnvalue_3)
      (bind _output_get (Variables|Default|SetbehaviorState "EB_Succeed"))
      (return _output_get)))
  (bind _output_get_2 (Variables|Default|SetbehaviorState "EB_Succeed"))
  (return _output_get_2))