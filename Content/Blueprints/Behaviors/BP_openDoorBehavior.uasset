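; BP_openDoorBehavior is a behavior for an RGBehaviorTreeComponent that lets an agent open its current storage, presumably a door, with a key.
; On Tick it checks the owner's inventory component for a BP_key and fails if none is held.
; With a key, it destroys the BP_agent's CurrentStorage actor, consumes one key, removes the BP_openDoor mood behavior and reports success.
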(fn Tick
  (params (deltaTime :type Float%20%28single-precision%29))
  (bind _m_ownercomp (Variables|Default|Getm_ownerComp))
  (bind _returnvalue (Components|GetOwner _m_ownercomp))
  (bind _returnvalue_2 (Actor|GetComponentbyClass _returnvalue "/Script/Simulation.InverntoryComponent"))
  (bind _returnvalue_3 (Class|InverntoryComponent|GetInventory _returnvalue_2 "/Game/Blueprints/interactables/Consumables/BP_key.BP_key_C"))
  (if (> _returnvalue_3 0)
    (bind _asbp_agent (Utilities|Casting|CastToBP_agent _returnvalue))
    (Actor|DestroyActor (Variables|/Script/Simulation.Agent|GetcurrentStorage _asbp_agent))
    (Class|InverntoryComponent|RemoveInventory _returnvalue_2 "/Game/Blueprints/interactables/Consumables/BP_key.BP_key_C" 1)
    (Class|RGBehaviorTreeComponent|RemoveMoodBehavior (Actor|GetComponentbyClass _returnvalue "/Script/Simulation.RGBehaviorTreeComponent") "/Game/Blueprints/Moods/BP_openDoor.BP_openDoor_C")
    (bind _output_get (Variables|Default|SetbehaviorState "EB_Succeed"))
    (return _output_get)
    (else
      (bind _output_get_2 (Variables|Default|SetbehaviorState "EB_Failed"))
      (return _output_get_2))))